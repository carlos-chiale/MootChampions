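; BP_PaintBomb is a paint-the-floor powerup that recolors the tiles around the player who touches it.
; Every Tick it polls its Collision component for overlapping BP_PaintFloorPlayer actors and takes the first one.
; A sphere overlap of ExplosionRadius, centered on that player rather than the bomb, gathers WorldStatic BP_Tile actors.
; Each tile receives the player's index and color through SetColor, then the bomb destroys itself.
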(event EventBeginPlay)

(event Collision|EventActorBeginOverlap
  (params (OtherActor :type Actor%20Object%20Reference)))

(event EventTick
  (params (DeltaSeconds :type Float%20%28single-precision%29))
  (CallFunction|ExplodePaintingBomb))

(fn ConstructionScript)

(fn ExplodePaintingBomb
  (bind _asbp_paint_floor_player (Utilities|Casting|CastToBP_PaintFloorPlayer (Utilities|Array|Get(acopy) (Collision|GetOverlappingActors (Variables|Default|GetCollision) "/Game/PaintTheFloor/Blueprints/BP_PaintFloorPlayer.BP_PaintFloorPlayer_C" :!class /Script/Engine.PrimitiveComponent))))
  (bind _outactors (Collision|SphereOverlapActors (Transformation|GetActorLocation _asbp_paint_floor_player) (Variables|Default|GetExplosionRadius) (Utilities|Array|MakeArray "ObjectTypeQuery1") "/Game/PaintTheFloor/Blueprints/BP_Tile.BP_Tile_C"))
  (for _array_element _outactors
    (bind _asbp_tile (Utilities|Casting|CastToBP_Tile _array_element))
    (Default|SetColor _asbp_tile (Variables|/Game/PaintTheFloor/Blueprints/BP_PaintFloorPlayer.BP_PaintFloorPlayer_C|GetIndex _asbp_paint_floor_player) (Variables|/Game/PaintTheFloor/Blueprints/BP_PaintFloorPlayer.BP_PaintFloorPlayer_C|GetTileColor _asbp_paint_floor_player)))
  (Actor|DestroyActor))