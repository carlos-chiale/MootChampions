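; BP_FreezeBomb is a Paint The Floor powerup that freezes every rival of the player who picks it up.
; Each Tick it runs FreezeRivals, which takes the first BP_PaintFloorPlayer overlapping its Collision as the collector.
; It then calls Freeze with TimeFreezed on all other players in the world, destroying itself inside that loop, so only when a rival exists.
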(event EventBeginPlay)

(event EventTick
  (params (DeltaSeconds :type Float%20%28single-precision%29))
  (CallFunction|FreezeRivals))

(fn ConstructionScript)

(fn FreezeRivals
  (bind _asbp_paint_floor_player (Utilities|Casting|CastToBP_PaintFloorPlayer (Utilities|Array|Get(acopy) (Collision|GetOverlappingActors (Variables|Default|GetCollision) "/Game/PaintTheFloor/Blueprints/BP_PaintFloorPlayer.BP_PaintFloorPlayer_C" :!class /Script/Engine.PrimitiveComponent))))
  (bind _output_get (LocalVariables|SetPlayerGetPowerUp _asbp_paint_floor_player))
  (bind _outactors (Actor|GetAllActorsOfClass "/Game/PaintTheFloor/Blueprints/BP_PaintFloorPlayer.BP_PaintFloorPlayer_C"))
  (for _array_element _outactors
    (if (!= _array_element _output_get)
      (Default|Freeze _array_element (Variables|Default|GetTimeFreezed))
      (Actor|DestroyActor))))