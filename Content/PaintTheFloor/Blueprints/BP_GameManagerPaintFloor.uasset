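; Game manager for the Paint the Floor minigame, running the match countdown, powerup spawns and end-of-match ranking.
; A one-second looping timer drives both countdowns, which Tick polls to drop a freeze bomb, random-radius paint bomb or roller above a random board tile.
; At time zero it ranks players by repeatedly taking the board's highest painted count, saves that to the game instance, pauses and shows the win widget.
; The win-count increment is left unconnected.
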(event EventBeginPlay
  (bind _returnvalue (Actor|GetActorOfClass "/Game/PaintTheFloor/Blueprints/BP_Board.BP_Board_C"))
  (Variables|Default|SetBoard _returnvalue)
  (Utilities|Time|SetTimerbyFunctionName 0 "Decrement" 1.0 true)
  (Variables|Powerups|SetTimeToAppearPowerups (Math|Random|RandomIntegerinRange (Variables|Powerups|GetMinSecondsToSpawnPowerup) (Variables|Powerups|GetMaxSecondsToSpawnPowerup))))

(event EventTick
  (params (DeltaSeconds :type Float%20%28single-precision%29))
  (bind _returnvalue (Game|GetPlayerController 0))
  (CallFunction|SpawnPowerups)
  (if (and (== (Variables|Tosetup|GetTimeInSeconds) 0) (not (Variables|Default|GetGameFinished)))
    (Variables|Default|SetGameFinished true)
    (Class|KismetSystemLibrary|PauseTimer 0 "Decrement")
    (bind _rankingout (CallFunction|GetRanking))
    (Variables|Default|SetFinalRanking _rankingout)
    (bind _asmy_game_instance (Utilities|Casting|CastToMyGameInstance (Game|GetGameInstance)))
    (for (_array_element _array_index) (Variables|Default|GetFinalRanking)
      (Utilities|Array|SetArrayElem (Variables|/Game/MyGameInstance.MyGameInstance_C|GetLastGameRank _asmy_game_instance) _array_index _array_element))
    (Input|SetInputModeGameandUI _returnvalue 0 "DoNotLock" false)
    (Variables|/Script/Engine.PlayerController|SetbShowMouseCursor _returnvalue true)
    (Game|SetGamePaused true)
    (bind _returnvalue_2 (UserInterface|CreateWidget "/Game/PaintTheFloor/Blueprints/UI/W_Win.W_Win_C"))
    (UserInterface|Viewport|AddtoViewport _returnvalue_2 0)))

(fn ConstructionScript)

(fn Decrement
  (Variables|Tosetup|SetTimeInSeconds (- (Variables|Tosetup|GetTimeInSeconds) 1))
  (Variables|Powerups|SetTimeToAppearPowerups (- (Variables|Powerups|GetTimeToAppearPowerups) 1)))

(fn GetRanking
  (LocalVariables|SetPaintedAux (Variables|/Game/PaintTheFloor/Blueprints/BP_Board.BP_Board_C|GetPainted (Variables|Default|GetBoard)))
  (while (> (LocalVariables|GetAux) 0)
    (Utilities|Array|SetArrayElem (LocalVariables|GetRanking) (LocalVariables|GetAuxIndexRanking) (.IndexOfMaxValue (Math|Integer|MaxOfIntArray (LocalVariables|GetPaintedAux))))
    (Utilities|Array|SetArrayElem (LocalVariables|GetPaintedAux) (.IndexOfMaxValue (Math|Integer|MaxOfIntArray (LocalVariables|GetPaintedAux))) -1)
    (LocalVariables|SetAux (- (LocalVariables|GetAux) 1))
    (LocalVariables|SetAuxIndexRanking (+ (LocalVariables|GetAuxIndexRanking) 1)))
  (return (LocalVariables|GetRanking)))

(fn SpawnPowerups
  (if (== (Variables|Powerups|GetTimeToAppearPowerups) 0)
    (Variables|Powerups|SetTimeToAppearPowerups (Math|Random|RandomIntegerinRange (Variables|Powerups|GetMinSecondsToSpawnPowerup) (Variables|Powerups|GetMaxSecondsToSpawnPowerup)))
    (bind _output_get (LocalVariables|SetSpawnLocation (+ (Transformation|GetActorLocation (.OutItem (Utilities|Array|Random (Variables|/Game/PaintTheFloor/Blueprints/BP_Board.BP_Board_C|GetTiles (Variables|Default|GetBoard))))) "0, 0,100.000000")))
    (switch int (Math|Random|RandomIntegerinRange 0 2)
      (:0
        (Game|SpawnActorfromClass "/Game/PaintTheFloor/Blueprints/Powerups/BP_FreezeBomb.BP_FreezeBomb_C" (Math|Conversions|ToTransform(Vector) _output_get) "Undefined" 0 0))
      (:1
        (bind _returnvalue (Game|SpawnActorfromClass "/Game/PaintTheFloor/Blueprints/Powerups/BP_PaintBomb.BP_PaintBomb_C" (Math|Conversions|ToTransform(Vector) _output_get) "Undefined" 0 0))
        (Variables|/Game/PaintTheFloor/Blueprints/Powerups/BP_PaintBomb.BP_PaintBomb_C|SetExplosionRadius _returnvalue (Math|Random|RandomFloatinRange (Variables|Bombpaint|GetMinBombRadius) (Variables|Bombpaint|GetMaxBombRadius))))
      (:2
        (Game|SpawnActorfromClass "/Game/PaintTheFloor/Blueprints/Powerups/BP_Roller.BP_Roller_C" (Math|Conversions|ToTransform(Vector) _output_get) "Undefined" 0 0)))))