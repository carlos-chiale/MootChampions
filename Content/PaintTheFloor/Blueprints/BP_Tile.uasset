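; BP_Tile is a floor tile in the Paint The Floor game that players claim by changing its color.
; On BeginPlay it caches the level's BP_Board actor.
; SetColor acts only when the player differs from the current owner, reporting the new and old owner to the board, swapping the tile mesh material and storing the new owner index.
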(event EventBeginPlay
  (bind _returnvalue (Actor|GetActorOfClass "/Game/PaintTheFloor/Blueprints/BP_Board.BP_Board_C"))
  (Variables|Default|SetBoard _returnvalue))

(event Collision|EventActorBeginOverlap
  (params (OtherActor :type Actor%20Object%20Reference)))

(event EventTick
  (params (DeltaSeconds :type Float%20%28single-precision%29)))

(fn ConstructionScript)

(fn SetColor
  (params (PlayerIndex :type Integer) (TileColor :type Material%20Instance%20Object%20Reference))
  (if (!= PlayerIndex (Variables|Default|GetIndexPlayerOwns))
    (Default|TiledPainted (Variables|Default|GetBoard) PlayerIndex (Variables|Default|GetIndexPlayerOwns))
    (Rendering|Material|SetMaterial (Variables|Default|GetTile) 0 TileColor)
    (Variables|Default|SetIndexPlayerOwns PlayerIndex)))