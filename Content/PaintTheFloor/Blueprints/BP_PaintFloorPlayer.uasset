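; Player character for a paint-the-floor game: its Index selects mesh and color, and a downward trace each Tick recolors the BP_Tile underneath.
; Jump triggers a tackle that stuns and launches overlapped players, while Escape or P opens the pause menu.
; Freeze, stun and speed boost use one-second looping countdown timers, with expiry checked on Tick.
; Boosting drives a velocity-based smear on the dynamic material, and freezing swaps in ice.
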(event OnComponentBeginOverlap(TackleCollision)
  (params (OverlappedComponent :type Primitive%20Component%20Object%20Reference) (OtherActor :type Actor%20Object%20Reference) (OtherComp :type Primitive%20Component%20Object%20Reference) (OtherBodyIndex :type Integer) (bFromSweep :type Boolean) (SweepResult :type Hit%20Result%20Structure%20%28by%20ref%29))
  ;[1 1 1] Tackle
  (bind _asbp_paint_floor_player (Utilities|Casting|CastToBP_PaintFloorPlayer OtherActor))
  (if (and (not (Variables|BP_PaintFloorPlayer_C|GetIsStunt _asbp_paint_floor_player)) (Variables|Default|GetIsTackling))
    (CallFunction|Stunt _asbp_paint_floor_player 5)
    (Character|LaunchCharacter _asbp_paint_floor_player (* (Variables|/Script/Engine.MovementComponent|GetVelocity (Variables|Character|GetCharacterMovement)) 7) false false)))

(event EventTick
  (params (DeltaSeconds :type Float%20%28single-precision%29))
  (bind _capsulecomponent (Variables|Collision|GetCapsuleComponent))
  (bind _returnvalue (Transformation|GetWorldLocation _capsulecomponent))
  ;[1 1 1] Paint floor
  (bind _outhit (Collision|LineTraceForObjects _returnvalue (+ _returnvalue (* (* (Math|Vector|GetUpVector (Transformation|GetWorldRotation _capsulecomponent)) -1) (Variables|Default|GetConstant))) (Utilities|Array|MakeArray "ObjectTypeQuery1") false 0 "None"))
  (bind _asbp_tile (Utilities|Casting|CastToBP_Tile (.HitActor (Collision|BreakHitResult _outhit))))
  (Default|SetColor _asbp_tile (Variables|Default|GetIndex) (Variables|Default|GetTileColor))
  (CallFunction|Unfreeze)
  (CallFunction|UnStunt)
  (CallFunction|DecreaseSpeed)
  (CallFunction|SpeedIncreasedMaterial))

(event EventBeginPlay
  (bind _returnvalue (Rendering|Material|CreateDynamicMaterialInstance (Variables|Character|GetMesh) 0 (Utilities|Select :Index (Variables|Default|GetIndex) :Option%200 "/Game/PaintTheFloor/Materials/MI_SmearTexture_Blue.MI_SmearTexture_Blue" :Option%201 "/Game/PaintTheFloor/Materials/MI_SmearTexture_Green.MI_SmearTexture_Green" :Option%202 "/Game/PaintTheFloor/Materials/MI_SmearTexture_Red.MI_SmearTexture_Red" :Option%203 "/Game/PaintTheFloor/Materials/MI_SmearTexture_Yellow.MI_SmearTexture_Yellow") "None" :!class /Script/Engine.PrimitiveComponent))
  (Variables|Default|SetM_Reference _returnvalue)
  (Utilities|Time|SetTimerbyFunctionName 0 "DecrementWhileFreezing" 1.0 true)
  (Utilities|Time|SetTimerbyFunctionName 0 "DecrementWhileSpeedIncreased" 1.0 true)
  (Utilities|Time|SetTimerbyFunctionName 0 "DecrementWhileStunning" 1.0 true))

(event Input|ActionEvents|InputActionJump
  (params (Key :type Key%20Structure))
  ;[1 1 1] Tackle
  (:Pressed
    (if (and (not (Variables|Default|GetIsFreeze)) (not (Variables|Default|GetIsTackling)))
      (Variables|Default|SetIsTackling true))))

(event Input|AxisEvents|InputAxisMoveForward
  (params (AxisValue :type Float%20%28single-precision%29))
  ;[1 1 1] Movement
  (if (not (or (Variables|Default|GetIsFreeze) (Variables|Default|GetIsStunt)))
    (Pawn|Input|AddMovementInput "90.000000, 0, 0" AxisValue false)))

(event Input|AxisEvents|InputAxisMoveRight
  (params (AxisValue :type Float%20%28single-precision%29))
  ;[1 1 1] Movement
  (if (not (or (Variables|Default|GetIsFreeze) (Variables|Default|GetIsStunt)))
    (Pawn|Input|AddMovementInput "0.000000,90.000000, 0" AxisValue false)))

(event Input|KeyboardEvents|P
  (params (Key :type Key%20Structure))
  (bind _returnvalue (Game|GetPlayerController 0))
  ;[1 1 1] Pause Game
  (:Pressed
    (Variables|/Script/Engine.PlayerController|SetbShowMouseCursor _returnvalue true)
    (bind _returnvalue_2 (UserInterface|CreateWidget "/Game/PauseMenu/W_PauseMenu.W_PauseMenu_C"))
    (UserInterface|Viewport|AddtoViewport _returnvalue_2 0)
    (Game|SetGamePaused true)
    (Input|SetInputModeUIOnly _returnvalue _returnvalue_2 "DoNotLock")))

(event Input|KeyboardEvents|Escape
  (params (Key :type Key%20Structure))
  (bind _returnvalue (Game|GetPlayerController 0))
  ;[1 1 1] Pause Game
  (:Pressed
    (Variables|/Script/Engine.PlayerController|SetbShowMouseCursor _returnvalue true)
    (bind _returnvalue_2 (UserInterface|CreateWidget "/Game/PauseMenu/W_PauseMenu.W_PauseMenu_C"))
    (UserInterface|Viewport|AddtoViewport _returnvalue_2 0)
    (Game|SetGamePaused true)
    (Input|SetInputModeUIOnly _returnvalue _returnvalue_2 "DoNotLock")))

(fn ConstructionScript)

(fn SetPlayerandColorbyIndex
  (bind _index (Variables|Default|GetIndex))
  (Class|SkinnedMeshComponent|SetSkeletalMesh (Variables|Character|GetMesh) (Utilities|Select :Index _index :Option%200 "/Game/Characters/CharacterTPose/BlueCharacter/TPoseBlueCharacter.TPoseBlueCharacter" :Option%201 "/Game/Characters/CharacterTPose/GreenCharacter/TPoseGreenCharacter.TPoseGreenCharacter" :Option%202 "/Game/Characters/CharacterTPose/RedCharacter/TPoseRedCharacter.TPoseRedCharacter" :Option%203 "/Game/Characters/CharacterTPose/YellowCharacter/TPoseYellowCharacter.TPoseYellowCharacter") true)
  (Variables|Default|SetTileColor (Utilities|Select :Index _index :Option%200 "/Game/PaintTheFloor/Materials/BlueTile.BlueTile" :Option%201 "/Game/PaintTheFloor/Materials/GreenTile.GreenTile" :Option%202 "/Game/PaintTheFloor/Materials/RedTile.RedTile" :Option%203 "/Game/PaintTheFloor/Materials/OrangeTile.OrangeTile")))

(fn Freeze
  (params (TimeToUnfreeze :type Integer))
  (Variables|Default|SetTimeToUnfreeze TimeToUnfreeze)
  (Variables|Default|SetIsFreeze true)
  (Rendering|Material|SetMaterial (Variables|Character|GetMesh) 0 "/Game/PaintTheFloor/Materials/MI_Ice.MI_Ice"))

(fn DecrementWhileFreezing
  (if (Variables|Default|GetIsFreeze)
    (Variables|Default|SetTimeToUnfreeze (- (Variables|Default|GetTimeToUnfreeze) 1))))

(fn IncrementVelocity
  (Variables|/Script/Engine.CharacterMovementComponent|SetMaxWalkSpeed (Variables|Character|GetCharacterMovement) 1.2e+03)
  (Variables|Default|SetIsSpeedIncremented true)
  (Variables|Default|SetTimeToPutMaxSpeedNormal 5))

(fn DecrementWhileSpeedIncreased
  (if (Variables|Default|GetIsSpeedIncremented)
    (Variables|Default|SetTimeToPutMaxSpeedNormal (- (Variables|Default|GetTimeToPutMaxSpeedNormal) 1))))

(fn Unfreeze
  (if (and (== (Variables|Default|GetTimeToUnfreeze) 0) (Variables|Default|GetIsFreeze))
    (Rendering|Material|SetMaterial (Variables|Character|GetMesh) 0 (Variables|Default|GetM_Reference))
    (Variables|Default|SetIsFreeze false)))

(fn DecreaseSpeed
  (if (and (== (Variables|Default|GetTimeToPutMaxSpeedNormal) 0) (Variables|Default|GetIsSpeedIncremented))
    (Variables|Default|SetIsSpeedIncremented false)
    (Variables|/Script/Engine.CharacterMovementComponent|SetMaxWalkSpeed (Variables|Character|GetCharacterMovement) 6e+02)
    (Rendering|Material|SetScalarParameterValue (Variables|Default|GetM_Reference) "Amount" 0.0 :!class /Script/Engine.MaterialInstanceDynamic)))

(fn Stunt
  (params (TimeToUnstunt :type Integer))
  (Variables|Default|SetTimeToUnstunt TimeToUnstunt)
  (Variables|Default|SetIsStunt true)
  (Components|Animation|PlayAnimation (Variables|Character|GetMesh) "/Game/Characters/AnimationsSequences/Hit.Hit" false)
  (Components|Animation|SetAnimationMode (Variables|Character|GetMesh) "AnimationBlueprint")
  (Components|Activation|Activate (Variables|Default|GetStuntStars) true))

(fn UnStunt
  (if (and (== (Variables|Default|GetTimeToUnstunt) 0) (Variables|Default|GetIsStunt))
    (Components|Activation|Deactivate (Variables|Default|GetStuntStars))
    (Variables|Default|SetIsStunt false)))

(fn DecrementWhileStunning
  (if (Variables|Default|GetIsStunt)
    (Variables|Default|SetTimeToUnstunt (- (Variables|Default|GetTimeToUnstunt) 1))))

(fn SpeedIncreasedMaterial
  (bind _m_reference (Variables|Default|GetM_Reference))
  (if (Variables|Default|GetIsSpeedIncremented)
    (Rendering|Material|SetVectorParameterValue _m_reference "Loc" (Math|Conversions|ToLinearColor(Vector) (* (Math|Vector|GetForwardVector (Variables|Collision|GetCapsuleComponent)) -1.0)) :!class /Script/Engine.MaterialInstanceDynamic)
    (Rendering|Material|SetScalarParameterValue _m_reference "Amount" (/ (Math|Vector|VectorLengthSquared (Variables|/Script/Engine.MovementComponent|GetVelocity (Variables|Character|GetCharacterMovement))) 9e+05) :!class /Script/Engine.MaterialInstanceDynamic)
    (Rendering|Material|SetVectorParameterValue _m_reference "Base Color" (Utilities|Select :Index (Variables|Default|GetIndex) :Option%200 "(R=0.000000,G=0.082035,B=0.672090,A=1.000000)" :Option%201 "(R=0.000000,G=0.450506,B=0.129966,A=1.000000)" :Option%202 "(R=0.413425,G=0.000000,B=0.000000,A=1.000000)" :Option%203 "(R=0.840880,G=0.829003,B=0.000000,A=1.000000)") :!class /Script/Engine.MaterialInstanceDynamic)))