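; AI-controlled character for the Dodge minigame that takes laser damage and dies when health runs out.
; Each laser hit starts a timed invulnerability, with a timeline flickering the mesh's Alpha material parameter.
; Tick refreshes the health bar and, outside invulnerability, triggers a one-time death that enables mesh physics, stops movement and hides the widgets.
; A player index selects the colored mesh and tile; movement decisions are not in this Blueprint.
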(event Custom|LaserHitAI
  (params (LaserTurretRelocationDamage :type Float%20%28single-precision%29))
  ;[1 1 1] Evento cuándo un laser colisiona con el jugador
  (Variables|Default|SetLaser%20Turret%20Relocation%20Damage LaserTurretRelocationDamage)
  (if (not (Variables|Default|GetInvulnerability))
    (Variables|Default|SetHealth (- (Variables|Default|GetHealth) (Variables|Default|GetLaser%20Turret%20Relocation%20Damage)))
    (if (not (Variables|Default|GetInvulnerability))
      (Variables|Default|SetInvulnerability true)
      (Utilities|Time|SetTimerbyFunctionName 0 "SetVulnerable" (Variables|Default|GetInvulnerabilityTime))
      (CallFunction|VulnerabilityStart))))

(event Custom|VulnerabilityEnd
  ;[1 1 1] Tintineo mientras se está invulnerable
  (Development|PrintString "desactivo")
  (Rendering|Material|SetScalarParameterValueonMaterials (Variables|Character|GetMesh) "Alpha" 0.0)
  (bind _flick (Timeline|Timeline_0 Stop)
    (:Update
      (Rendering|Material|SetScalarParameterValueonMaterials (Variables|Character|GetMesh) "Alpha" _flick))))

(event Custom|VulnerabilityStart
  ;[1 1 1] Tintineo mientras se está invulnerable
  (Development|PrintString "activo")
  (bind _flick (Timeline|Timeline_0 Play)
    (:Update
      (Rendering|Material|SetScalarParameterValueonMaterials (Variables|Character|GetMesh) "Alpha" _flick))))

(event EventBeginPlay
  (Variables|/Script/Engine.CharacterMovementComponent|SetMaxWalkSpeed (Variables|Character|GetCharacterMovement) 5.5e+02))

(event EventTick
  (params (DeltaSeconds :type Float%20%28single-precision%29))
  ;[1 1 1] Indicador de vida y número de jugador
  (CallFunction|HealthUI)
  (CallFunction|PlayerNumberText)
  (Transformation|SetWorldRotation (Variables|Default|GetPlayerNumber) (Math|Rotator|MakeRotator 0.0 0.0 1.8e+02) false false)
  (if (not (Variables|Default|GetInvulnerability))
    ;[1 1 1] Muerte
    (if (<= (Variables|Default|GetHealth) 0.0)
      (Utilities|FlowControl|DoOnce false
        (:Completed
          (CallFunction|Death))))))

(fn ConstructionScript)

(fn HealthUI
  (bind _ashealth_bar (Utilities|Casting|CastToHealthBar (UserInterface|GetUserWidgetObject (Variables|Default|GetHealthBar))))
  (Progress|SetPercent (Variables|/Game/MinijuegoDodge/Blueprint/UIwidgets/HealthBar.HealthBar_C|GetProgressBar_0 _ashealth_bar) (/ (Variables|Default|GetHealth) 1e+02))
  (Transformation|SetWorldRotation (Variables|Default|GetHealthBar) (Math|Rotator|MakeRotator 0.0 0.0 1.8e+02) false false))

(fn Death
  (Physics|SetSimulatePhysics (Variables|Character|GetMesh) true)
  (Pawn|Components|CharacterMovement|DisableMovement (Variables|Character|GetCharacterMovement))
  (Rendering|SetVisibility (Variables|Default|GetPlayerNumber) false false)
  (Rendering|SetVisibility (Variables|Default|GetHealthBar) false false)
  (Collision|SetCollisionEnabled (Variables|Collision|GetCapsuleComponent) "PhysicsOnly")
  (Variables|Default|SetAlive false))

(fn PlayerNumberText
  (bind _asplayer_number (Utilities|Casting|CastToPlayerNumber (UserInterface|GetUserWidgetObject (Variables|Default|GetPlayerNumber))))
  (return))

(fn TimerWidget
  (bind _returnvalue (UserInterface|CreateWidget "/Game/MinijuegoDodge/Blueprint/UIwidgets/TimeCount.TimeCount_C" (Game|GetPlayerController -1)))
  (UserInterface|Viewport|AddtoPlayerScreen _returnvalue))

(fn SetVulnerable
  (Variables|Default|SetInvulnerability false)
  (CallFunction|VulnerabilityEnd))

(fn SetPlayerandColorbyIndex
  (bind _index (Variables|Default|GetIndex))
  (Class|SkinnedMeshComponent|SetSkeletalMesh (Variables|Character|GetMesh) (Utilities|Select :Index _index :Option%200 "/Game/Characters/CharacterTPose/BlueCharacter/TPoseBlueCharacter.TPoseBlueCharacter" :Option%201 "/Game/Characters/CharacterTPose/GreenCharacter/TPoseGreenCharacter.TPoseGreenCharacter" :Option%202 "/Game/Characters/CharacterTPose/RedCharacter/TPoseRedCharacter.TPoseRedCharacter" :Option%203 "/Game/Characters/CharacterTPose/YellowCharacter/TPoseYellowCharacter.TPoseYellowCharacter") true)
  (Variables|Default|SetTileColor (Utilities|Select :Index _index :Option%200 "/Game/PaintTheFloor/Materials/BlueTile.BlueTile" :Option%201 "/Game/PaintTheFloor/Materials/GreenTile.GreenTile" :Option%202 "/Game/PaintTheFloor/Materials/RedTile.RedTile" :Option%203 "/Game/PaintTheFloor/Materials/OrangeTile.OrangeTile")))