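; Rotating laser turret hazard for the dodge minigame that damages players hit by its laser.
; After delays, it stretches a placeholder cylinder and hit trigger forward, plus a wide trigger notifying characters for AI jumping.
; A timeline sweeps it by a yaw offset, optionally reverses once, then explodes and destroys it.
; Touching the body fires a push impulse; beam particle and spark effects are disabled by constant branches.
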(event OnComponentBeginOverlap(LaserColissionToJumpAi)
  (params (OverlappedComponent :type Primitive%20Component%20Object%20Reference) (OtherActor :type Actor%20Object%20Reference) (OtherComp :type Primitive%20Component%20Object%20Reference) (OtherBodyIndex :type Integer) (bFromSweep :type Boolean) (SweepResult :type Hit%20Result%20Structure%20%28by%20ref%29))
  (bind _asdodge_player_character (Utilities|Casting|CastToDodgePlayerCharacter OtherActor))
  (Variables|Default|SetAs%20Player%20Character _asdodge_player_character)
  (Default|LaserColisiontoJumpAi (Variables|Default|GetAs%20Player%20Character)))

(event OnComponentBeginOverlap(LaserColission)
  (params (OverlappedComponent :type Primitive%20Component%20Object%20Reference) (OtherActor :type Actor%20Object%20Reference) (OtherComp :type Primitive%20Component%20Object%20Reference) (OtherBodyIndex :type Integer) (bFromSweep :type Boolean) (SweepResult :type Hit%20Result%20Structure%20%28by%20ref%29))
  ;[1 1 1] Activar hit con personaje e IA
  (bind _asdodge_player_character (Utilities|Casting|CastToDodgePlayerCharacter OtherActor))
  (Variables|Default|SetAs%20Player%20Character _asdodge_player_character)
  (Default|LaserHitPlayer (Variables|Default|GetAs%20Player%20Character) (Variables|Default|GetDamage)))

(event OnComponentBeginOverlap(BoxColiderMesh)
  (params (OverlappedComponent :type Primitive%20Component%20Object%20Reference) (OtherActor :type Actor%20Object%20Reference) (OtherComp :type Primitive%20Component%20Object%20Reference) (OtherBodyIndex :type Integer) (bFromSweep :type Boolean) (SweepResult :type Hit%20Result%20Structure%20%28by%20ref%29))
  (bind _returnvalue (Transformation|GetActorLocation))
  (bind (_x _y _z) (Math|Vector|BreakVector _returnvalue))
  ;[1 1 1] Empuje al tocar la torreta
  (Utilities|Casting|CastToThirdPersonCharacter OtherActor)
  ;;[1 1 1] Activar empuje
  (if true
    (Class|RadialForceComponent|FireImpulse (Variables|Default|GetExplosion))
    ;;[1 1 1] Activar particulas
    (if false
      (bind _returnvalue_2 (Effects|SpawnEmitteratLocation "/Game/StarterContent/Particles/P_Sparks.P_Sparks" (Math|Vector|MakeVector _x _y (+ _z 3e+01))))
      (Audio|PlaySoundatLocation "/Game/MinijuegoDodge/Sounds/Electricidad.Electricidad" _returnvalue "0, 0, 0" 1.0 1.0 0.0 0 0 0)
      (Utilities|FlowControl|Delay 1.0)
      (Components|DestroyComponent _returnvalue_2))))

(event EventBeginPlay
  ;[1 1 1] Crear beam + trigger
  (Collision|SetCollisionEnabled (Variables|Default|GetLaserColission) "NoCollision")
  (bind _output_get (Variables|Default|SetBeamEndPoint (Utilities|LaserEndPoint)))
  ;;[1 1 1] Activar partícula de láser
  (if false
    (CallFunction|CreateParticle (Transformation|GetWorldLocation (Variables|Default|GetLaserStartPoint)) _output_get))
  ;;[1 1 1] Delay para disparar el rayo
  (Utilities|FlowControl|Delay 1.0)
  ;;[1 1 1] Alargar el trigger box y el placeholder del láser
  (CallFunction|ScaleTriggerBox (Variables|Default|GetBeamEndPoint))
  (CallFunction|ScaleCylinder (Variables|Default|GetBeamEndPoint))
  (Collision|SetCollisionEnabled (Variables|Default|GetLaserColission) "QueryAndPhysics")
  (Variables|Default|SetInitRotation (Transformation|GetActorRotation))
  ;;[1 1 1] Delay para rotar/trasladarse
  (Utilities|FlowControl|Delay 1.0)
  (CallFunction|ScaleTriggerBoxJumpAi (Variables|Default|GetBeamEndPoint))
  ;;[1 1 1] Rotar la torreta
  (bind _turretrotation (Timeline|TimelineRotation Play)
    (:Update
      (Transformation|SetRelativeRotation (Variables|Transformation|GetRootComponent) (Math|Rotator|Lerp(Rotator) (Variables|Default|GetInitRotation) (Utilities|MakeRotator) _turretrotation) false false))
    (:Finished
      (if (Variables|Default|GetReverseRotation)
        (Variables|Default|SetReverseRotation false)
        (Utilities|FlowControl|Delay (Variables|Default|GetReverseWait))
        (Timeline|TimelineRotation ReverseFromEnd)
        (else
          ;;[1 1 1] Crear partículas de explosión
          (Utilities|FlowControl|Delay 1.0)
          (CallFunction|MakeExplosion)
          ;;[1 1 1] Destruir la torreta al finalizar la rotación
          (Actor|DestroyActor))))))

(fn ConstructionScript)

(fn CreateBeam
  (params (StartLocation :type Vector) (EndLocation :type Vector))
  (bind _returnvalue (Effects|SpawnEmitteratLocation "/Game/MinijuegoDodge/Textures/LaserParticles.LaserParticles" StartLocation))
  (bind _output_get (Variables|Default|SetLaserBeam _returnvalue))
  (Class|ParticleSystemComponent|SetBeamEndPoint _output_get 0 EndLocation))

(fn ScaleTriggerBox
  (params (EndLocation :type Vector))
  (bind _laserstartpoint (Variables|Default|GetLaserStartPoint))
  (bind _lasercolission (Variables|Default|GetLaserColission))
  (bind _returnvalue (Transformation|GetWorldLocation _laserstartpoint))
  (bind _returnvalue_2 (- EndLocation _returnvalue))
  (bind _returnvalue_3 (Math|Vector|VectorLength _returnvalue_2))
  (bind _returnvalue_4 (/ _returnvalue_3 2.0))
  (Transformation|SetRelativeScale3D (Variables|Default|GetLaserColission) (Math|Vector|MakeVector _returnvalue_4 1.0 1.0))
  (Transformation|SetRelativeLocation _lasercolission (+ (Variables|/Script/Engine.SceneComponent|GetRelativeLocation _lasercolission) (Math|Vector|MakeVector _returnvalue_4 0.0 0.0)) false false))

(fn ScaleCylinder
  (params (EndLocation :type Vector))
  (bind _laserplaceholder (Variables|Default|GetLaserPlaceholder))
  (bind _laserplaceholder_2 (Variables|Default|GetLaserPlaceholder))
  (bind _returnvalue (Transformation|GetWorldScale _laserplaceholder_2))
  (bind (_x _y) (Math|Vector|BreakVector _returnvalue))
  (Transformation|SetRelativeScale3D (Variables|Default|GetLaserPlaceholder) (Math|Vector|MakeVector _x _y 5e+01))
  (Transformation|SetRelativeLocation _laserplaceholder (+ (Variables|/Script/Engine.SceneComponent|GetRelativeLocation _laserplaceholder) (Math|Vector|MakeVector (/ (Math|Vector|VectorLength (- EndLocation (Transformation|GetWorldLocation (Variables|Default|GetLaserStartPoint)))) 2.0) 0.0 0.0)) false false))

(fn CreateParticle
  (params (Start :type Vector) (End :type Vector))
  (bind (_outhit _returnvalue) (Collision|LineTraceByChannel Start End "TraceTypeQuery1" false 0 "None"))
  (if _returnvalue
    (Variables|Default|SetBeamEndPoint (.Location (Collision|BreakHitResult _outhit))))
  (CallFunction|CreateBeam (Transformation|GetWorldLocation (Variables|Default|GetLaserStartPoint)) (Variables|Default|GetBeamEndPoint)))

(fn MakeExplosion
  (Effects|SpawnEmitteratLocation "/Game/StarterContent/Particles/P_Explosion.P_Explosion" (Transformation|GetActorLocation)))

(fn ScaleTriggerBoxJumpAi
  (params (EndLocation :type Vector))
  (bind _laserstartpoint (Variables|Default|GetLaserStartPoint))
  (bind _lasercolissiontojumpai (Variables|Default|GetLaserColissionToJumpAi))
  (bind _returnvalue (Transformation|GetWorldLocation _laserstartpoint))
  (bind _returnvalue_2 (- EndLocation _returnvalue))
  (bind _returnvalue_3 (Math|Vector|VectorLength _returnvalue_2))
  (bind _returnvalue_4 (/ _returnvalue_3 2.0))
  (Transformation|SetRelativeScale3D (Variables|Default|GetLaserColissionToJumpAi) (Math|Vector|MakeVector _returnvalue_4 45.0 1.0))
  (Transformation|SetRelativeLocation _lasercolissiontojumpai (+ (Variables|/Script/Engine.SceneComponent|GetRelativeLocation _lasercolissiontojumpai) (Math|Vector|MakeVector _returnvalue_4 0.0 0.0)) false false))