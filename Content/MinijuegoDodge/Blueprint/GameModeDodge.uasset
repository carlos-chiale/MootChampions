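; Game mode for the Dodge minigame, running a timed elimination match between human and AI players.
; BeginPlay places GameInstance players at PlayerStarts, spawning AI with a behavior tree, then shows instructions and pauses.
; A one-second Delay on Tick drives the countdown, ending the match at zero or one survivor.
; The survivor, or top of a four-player health sort, gains a GameInstance win before movement stops and the win screen appears.
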(event EventBeginPlay
  (CallFunction|AssignPlayers)
  (Game|SetGamePaused true))

(event EventTick
  (params (DeltaSeconds :type Float%20%28single-precision%29))
  (Utilities|FlowControl|Delay 1.0)
  (CallFunction|DecrementTimeCount)
  (CallFunction|EndMatchifTimeCountIs0)
  (CallFunction|EndMatchifPlayerCountIs1)
  (if (Variables|Default|GetEndedMatch)
    (Utilities|FlowControl|DoOnce false
      (:Completed
        (CallFunction|AnnounceWinners)
        (CallFunction|DisablePlayerMovement)))))

(fn ConstructionScript)

(fn NametoInt
  (params (PlayerStart :type Player%20Start%20Object%20Reference))
  (return (Math|Conversions|ToInteger(Byte) (Utilities|String|ToString(Name) (Variables|/Script/Engine.PlayerStart|GetPlayerStartTag PlayerStart)))))

(fn CreateTimerWidget
  (bind _returnvalue (UserInterface|CreateWidget "/Game/MinijuegoDodge/Blueprint/UIwidgets/TimeCount.TimeCount_C" (Game|GetPlayerController -1)))
  (UserInterface|Viewport|AddtoPlayerScreen _returnvalue))

(fn RunTimeCount
  (Variables|Default|SetTimeToEndMinigame (Variables|Default|GetTimeToEndMinigame)))

(fn DecrementTimeCount
  (if (> (Variables|Default|GetTimeToEndMinigame) 0.0)
    (if (not (Variables|Default|GetEndedMatch))
      (if (Variables|Default|GetStartedMatch)
        (bind _result (Math|Float|DecrementFloat (Variables|Default|GetTimeToEndMinigame))
          (:%20%20
            (Variables|Default|SetTimeToEndMinigame _result)))))))

(fn EndMatchifPlayerCountIs1
  (if (<= (Variables|Default|GetPlayersAliveCount) 1)
    (if (not (Variables|Default|GetEndedMatch))
      (if (Variables|Default|GetStartedMatch)
        (Variables|Default|SetEndedMatch true)
        (CallFunction|MakeWinnersifPlayerCountsIs1)))))

(fn EndMatchifTimeCountIs0
  (if (<= (Variables|Default|GetTimeToEndMinigame) 0.0)
    (if (not (Variables|Default|GetEndedMatch))
      (if (Variables|Default|GetStartedMatch)
        (Variables|Default|SetEndedMatch true)
        (CallFunction|MakeWinnersifTimeIs0)))))

(fn MakeWinnersifTimeIs0
  (bind _outactors (Actor|GetAllActorsOfClass "/Game/MinijuegoDodge/Blueprint/DodgePlayerCharacter.DodgePlayerCharacter_C"))
  (bind _dodgeplayersranked (CallFunction|Sort _outactors))
  (for (_array_element _array_index) _dodgeplayersranked
    (bind _asdodge_player_character (Utilities|Casting|CastToDodgePlayerCharacter _array_element))
    (bind _asmy_game_instance (Utilities|Casting|CastToMyGameInstance (Game|GetGameInstance)))
    (Utilities|Array|SetArrayElem (Variables|/Game/MyGameInstance.MyGameInstance_C|GetLastGameRank _asmy_game_instance) _array_index (Variables|/Game/MinijuegoDodge/Blueprint/DodgePlayerCharacter.DodgePlayerCharacter_C|GetIndex _asdodge_player_character)))
  (Utilities|Array|SetArrayElem (Variables|/Game/MyGameInstance.MyGameInstance_C|GetPlayers _asmy_game_instance) (Utilities|Array|Get(acopy) (Variables|/Game/MyGameInstance.MyGameInstance_C|GetLastGameRank _asmy_game_instance)) (Utilities|Struct|MakePlayerStruct (.SkeletalMesh (Utilities|Struct|BreakPlayerStruct (Utilities|Array|Get(acopy) (Variables|/Game/MyGameInstance.MyGameInstance_C|GetPlayers _asmy_game_instance) (Utilities|Array|Get(acopy) (Variables|/Game/MyGameInstance.MyGameInstance_C|GetLastGameRank _asmy_game_instance))))) (.PlayerId (Utilities|Struct|BreakPlayerStruct (Utilities|Array|Get(acopy) (Variables|/Game/MyGameInstance.MyGameInstance_C|GetPlayers _asmy_game_instance) (Utilities|Array|Get(acopy) (Variables|/Game/MyGameInstance.MyGameInstance_C|GetLastGameRank _asmy_game_instance))))) (.IsHuman (Utilities|Struct|BreakPlayerStruct (Utilities|Array|Get(acopy) (Variables|/Game/MyGameInstance.MyGameInstance_C|GetPlayers _asmy_game_instance) (Utilities|Array|Get(acopy) (Variables|/Game/MyGameInstance.MyGameInstance_C|GetLastGameRank _asmy_game_instance))))) (+ (.Wins (Utilities|Struct|BreakPlayerStruct (Utilities|Array|Get(acopy) (Variables|/Game/MyGameInstance.MyGameInstance_C|GetPlayers _asmy_game_instance) (Utilities|Array|Get(acopy) (Variables|/Game/MyGameInstance.MyGameInstance_C|GetLastGameRank _asmy_game_instance))))) 1) (.Color (Utilities|Struct|BreakPlayerStruct (Utilities|Array|Get(acopy) (Variables|/Game/MyGameInstance.MyGameInstance_C|GetPlayers _asmy_game_instance) (Utilities|Array|Get(acopy) (Variables|/Game/MyGameInstance.MyGameInstance_C|GetLastGameRank _asmy_game_instance))))))))

(fn AnnounceWinners
  (if (Variables|Default|GetStartedMatch)
    (CallFunction|CreateWinnerScreenWidget)
    (CallFunction|EnableMouse)))

(fn CreateWinnerScreenWidget
  (bind _returnvalue (UserInterface|CreateWidget "/Game/MinijuegoDodge/Blueprint/UIwidgets/DodgeWinScreen.DodgeWinScreen_C" (Game|GetPlayerController -1)))
  (UserInterface|Viewport|AddtoPlayerScreen _returnvalue))

(fn DisablePlayerMovement
  (bind _outactors (Actor|GetAllActorsOfClass "/Game/MinijuegoDodge/Blueprint/DodgePlayerCharacter.DodgePlayerCharacter_C"))
  (for _array_element _outactors
    (Pawn|Components|CharacterMovement|DisableMovement (Variables|/Script/Engine.Character|GetCharacterMovement _array_element))))

(fn EnableMouse
  (bind _returnvalue (Game|GetPlayerController 0))
  (Input|SetInputModeUIOnly _returnvalue 0 "DoNotLock")
  (Variables|/Script/Engine.PlayerController|SetbShowMouseCursor _returnvalue true))

(fn ChoosePlayerStart
  (params (Player :type Controller%20Object%20Reference))
  (return 0))

(fn CreateControllers)

(fn GetDefaultPawnClassforController
  (params (InController :type Controller%20Object%20Reference))
  (bind _returnvalue (|CallParentFunction 0))
  (return _returnvalue))

(fn SetSkeletalMeshtoPlayer1
  (Class|SkinnedMeshComponent|SetSkeletalMesh (Variables|/Script/Engine.Character|GetMesh (Game|GetPlayerCharacter 0)) (Utilities|Array|Get(acopy) (Variables|Default|GetPlayerSkeletalMesh)) true))

(fn AssignPlayers
  (bind _returnvalue (Game|GetPlayerController 0))
  (bind _outactors (Actor|GetAllActorsOfClass "/Script/Engine.PlayerStart"))
  (Variables|Default|SetPlayerStartArray _outactors)
  (bind _asmy_game_instance (Utilities|Casting|CastToMyGameInstance (Game|GetGameInstance)))
  (for _array_element (Variables|/Game/MyGameInstance.MyGameInstance_C|GetPlayers _asmy_game_instance)
    (LocalVariables|SetSkeletalMesh (.SkeletalMesh (Utilities|Struct|BreakPlayerStruct _array_element)))
    (LocalVariables|SetPlayerId (.PlayerId (Utilities|Struct|BreakPlayerStruct _array_element)))
    (LocalVariables|SetIsHuman (.IsHuman (Utilities|Struct|BreakPlayerStruct _array_element)))
    (if (!= (LocalVariables|GetPlayerId) 0)
      (if (LocalVariables|GetIsHuman)
        ;[1 1 1] Human player
        (Class|GameplayStatics|CreatePlayer (LocalVariables|GetPlayerId))
        (Transformation|SetActorTransform (Game|Player|GetPlayerPawn (LocalVariables|GetPlayerId)) (Math|Conversions|ToTransform(Vector) (Transformation|GetActorLocation (Utilities|Array|Get(acopy) (Variables|Default|GetPlayerStartArray) (Variables|Default|GetIndexStartingPoints)))))
        (Development|PrintString (Utilities|String|ToString(Integer) (Variables|Default|GetIndexStartingPoints)) true true "(R=0.000000,G=0.660000,B=1.000000,A=1.000000)" 2e+01)
        (Variables|Default|SetIndexStartingPoints (+ (Variables|Default|GetIndexStartingPoints) 1))
        (Variables|Default|SetAmountOfHumanPlayers (+ (Variables|Default|GetAmountOfHumanPlayers) 1))
        (else
          ;[1 1 1] AI player
          (bind _returnvalue_2 (AI|SpawnAIFromClass "/Game/MinijuegoDodge/Blueprint/DodgePlayerCharacter.DodgePlayerCharacter_C" "/Game/MinijuegoDodge/Blueprint/AI/BTDodge.BTDodge" (Transformation|GetActorLocation (Utilities|Array|Get(acopy) (Variables|Default|GetPlayerStartArray) (Variables|Default|GetIndexStartingPoints))) "0, 0, 0" false 0))
          (Variables|Default|SetIndexStartingPoints (+ (Variables|Default|GetIndexStartingPoints) 1))
          (bind _asdodge_player_character (Utilities|Casting|CastToDodgePlayerCharacter _returnvalue_2))
          (Variables|/Game/MinijuegoDodge/Blueprint/DodgePlayerCharacter.DodgePlayerCharacter_C|SetIsHuman _asdodge_player_character false)))
      (else
        (Transformation|SetActorLocation (Game|Player|GetPlayerPawn 0) (Transformation|GetActorLocation (Utilities|Array|Get(acopy) (Variables|Default|GetPlayerStartArray))) false false))))
  (bind _outactors_2 (Actor|GetAllActorsOfClass "/Game/MinijuegoDodge/Blueprint/DodgePlayerCharacter.DodgePlayerCharacter_C"))
  (for (_array_element_2 _array_index) _outactors_2
    (Variables|/Game/MinijuegoDodge/Blueprint/DodgePlayerCharacter.DodgePlayerCharacter_C|SetIndex _array_element_2 _array_index)
    (Default|SetPlayerandColorbyIndex _array_element_2))
  (Input|SetInputModeGameandUI _returnvalue 0 "DoNotLock" false)
  (Variables|/Script/Engine.PlayerController|SetbShowMouseCursor _returnvalue true)
  (Game|SetGamePaused false)
  (bind _returnvalue_3 (UserInterface|CreateWidget "/Game/MinijuegoDodge/Blueprint/UIwidgets/DodgeInstructionsScreen.DodgeInstructionsScreen_C"))
  (UserInterface|Viewport|AddtoViewport _returnvalue_3 0))

(fn MakeWinnersifPlayerCountsIs1
  (bind _outactors (Actor|GetAllActorsOfClass "/Game/MinijuegoDodge/Blueprint/DodgePlayerCharacter.DodgePlayerCharacter_C"))
  (for _array_element _outactors
    (if (Variables|/Game/MinijuegoDodge/Blueprint/DodgePlayerCharacter.DodgePlayerCharacter_C|GetAlive _array_element)
      (bind _asmy_game_instance (Utilities|Casting|CastToMyGameInstance (Game|GetGameInstance)))
      (Utilities|Array|SetArrayElem (Variables|/Game/MyGameInstance.MyGameInstance_C|GetLastGameRank _asmy_game_instance) 0 (Variables|/Game/MinijuegoDodge/Blueprint/DodgePlayerCharacter.DodgePlayerCharacter_C|GetIndex _array_element))
      (Utilities|Array|SetArrayElem (Variables|/Game/MyGameInstance.MyGameInstance_C|GetPlayers _asmy_game_instance) (Variables|/Game/MinijuegoDodge/Blueprint/DodgePlayerCharacter.DodgePlayerCharacter_C|GetIndex _array_element) (Utilities|Struct|MakePlayerStruct (.SkeletalMesh (Utilities|Struct|BreakPlayerStruct (Utilities|Array|Get(acopy) (Variables|/Game/MyGameInstance.MyGameInstance_C|GetPlayers _asmy_game_instance) (Variables|/Game/MinijuegoDodge/Blueprint/DodgePlayerCharacter.DodgePlayerCharacter_C|GetIndex _array_element)))) (.PlayerId (Utilities|Struct|BreakPlayerStruct (Utilities|Array|Get(acopy) (Variables|/Game/MyGameInstance.MyGameInstance_C|GetPlayers _asmy_game_instance) (Variables|/Game/MinijuegoDodge/Blueprint/DodgePlayerCharacter.DodgePlayerCharacter_C|GetIndex _array_element)))) (.IsHuman (Utilities|Struct|BreakPlayerStruct (Utilities|Array|Get(acopy) (Variables|/Game/MyGameInstance.MyGameInstance_C|GetPlayers _asmy_game_instance) (Variables|/Game/MinijuegoDodge/Blueprint/DodgePlayerCharacter.DodgePlayerCharacter_C|GetIndex _array_element)))) (+ (.Wins (Utilities|Struct|BreakPlayerStruct (Utilities|Array|Get(acopy) (Variables|/Game/MyGameInstance.MyGameInstance_C|GetPlayers _asmy_game_instance) (Variables|/Game/MinijuegoDodge/Blueprint/DodgePlayerCharacter.DodgePlayerCharacter_C|GetIndex _array_element)))) 1) (.Color (Utilities|Struct|BreakPlayerStruct (Utilities|Array|Get(acopy) (Variables|/Game/MyGameInstance.MyGameInstance_C|GetPlayers _asmy_game_instance) (Variables|/Game/MinijuegoDodge/Blueprint/DodgePlayerCharacter.DodgePlayerCharacter_C|GetIndex _array_element)))))))))

(fn ComparatorPlayersHealth
  (params (ObjectA :type Object%20Object%20Reference) (ObjectB :type Object%20Object%20Reference))
  (bind _asdodge_player_character (Utilities|Casting|CastToDodgePlayerCharacter ObjectA))
  (bind _asdodge_player_character_2 (Utilities|Casting|CastToDodgePlayerCharacter ObjectB))
  (Math|Float|CompareFloat (Variables|/Game/MinijuegoDodge/Blueprint/DodgePlayerCharacter.DodgePlayerCharacter_C|GetHealth _asdodge_player_character) (Variables|/Game/MinijuegoDodge/Blueprint/DodgePlayerCharacter.DodgePlayerCharacter_C|GetHealth _asdodge_player_character_2)
    (:>
      (return true))
    (:==
      (return true))
    (:<
      (return false))))

(fn Sort
  (params (DodgePlayers :type Array%20of%20Dodge%20Player%20Character%20Object%20References))
  (while (< (LocalVariables|GetIndex) 4)
    (while (< (LocalVariables|GetIndex2) 4)
      (if (and (not (Utilities|Array|Get(acopy) (LocalVariables|GetAdded) (LocalVariables|GetIndex2))) (>= (Variables|/Game/MinijuegoDodge/Blueprint/DodgePlayerCharacter.DodgePlayerCharacter_C|GetHealth (Utilities|Array|Get(acopy) DodgePlayers (LocalVariables|GetIndex2))) (LocalVariables|GetMaxHealthAux)))
        (LocalVariables|SetDodgePlayerAux (Utilities|Array|Get(acopy) DodgePlayers (LocalVariables|GetIndex2)))
        (LocalVariables|SetIndexAux (LocalVariables|GetIndex2))
        (LocalVariables|SetMaxHealthAux (Variables|/Game/MinijuegoDodge/Blueprint/DodgePlayerCharacter.DodgePlayerCharacter_C|GetHealth (Utilities|Array|Get(acopy) DodgePlayers (LocalVariables|GetIndex2)))))
      (LocalVariables|SetIndex2 (+ (LocalVariables|GetIndex2) 1)))
    (Utilities|Array|SetArrayElem (LocalVariables|GetReturnDodgePlayers) (LocalVariables|GetIndex) (LocalVariables|GetDodgePlayerAux))
    (Utilities|Array|SetArrayElem (LocalVariables|GetAdded) (LocalVariables|GetIndexAux) true)
    (LocalVariables|SetMaxHealthAux -1e+03)
    (LocalVariables|SetIndexAux -1)
    (LocalVariables|SetIndex (+ (LocalVariables|GetIndex) 1))
    (LocalVariables|SetIndex2 0))
  (return (LocalVariables|GetReturnDodgePlayers)))