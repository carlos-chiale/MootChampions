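; BP_SelectPlayerPlayer is the per-controller actor for the player selection screen, letting each player join or leave.
; On BeginPlay it caches the MyGameInstance.
; Pressing Start passes its player controller ID to the game instance's AddPlayer, and pressing Cancel passes it to DeletePlayer.
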(event EventBeginPlay
  (bind _asmy_game_instance (Utilities|Casting|CastToMyGameInstance (Game|GetGameInstance)))
  (Variables|Default|SetMyGameInstance _asmy_game_instance))

(event Collision|EventActorBeginOverlap
  (params (OtherActor :type Actor%20Object%20Reference)))

(event EventTick
  (params (DeltaSeconds :type Float%20%28single-precision%29)))

(event Input|ActionEvents|InputActionStart
  (params (Key :type Key%20Structure :default "None"))
  (:Pressed
    (bind _asplayer_controller (Utilities|Casting|CastToPlayerController (Pawn|GetController)))
    (Default|AddPlayer (Variables|Default|GetMyGameInstance) (Class|GameplayStatics|GetPlayerControllerID _asplayer_controller))))

(event Input|ActionEvents|InputActionCancel
  (params (Key :type Key%20Structure :default "None"))
  (:Pressed
    (bind _asplayer_controller (Utilities|Casting|CastToPlayerController (Pawn|GetController)))
    (Default|DeletePlayer (Variables|Default|GetMyGameInstance) (Class|GameplayStatics|GetPlayerControllerID _asplayer_controller))))

(fn ConstructionScript)