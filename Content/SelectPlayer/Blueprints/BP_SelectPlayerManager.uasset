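; BP_SelectPlayerManager is a player-select manager that makes the Green, Red and Orange characters dance when their player slot is human.
; BeginPlay caches MyGameInstance, and Tick polls the IsHuman flag of Players entries 1 to 3 through one function per colour.
; A per-character boolean ensures each looping animation, a unique dance or the shared breathing idle, restarts only when that state changes.
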(event EventBeginPlay
  (bind _asmy_game_instance (Utilities|Casting|CastToMyGameInstance (Game|GetGameInstance)))
  (Variables|Default|SetGameInstance _asmy_game_instance))

(event Collision|EventActorBeginOverlap
  (params (OtherActor :type Actor%20Object%20Reference)))

(event EventTick
  (params (DeltaSeconds :type Float%20%28single-precision%29))
  (CallFunction|GreenDancing)
  (CallFunction|RedDancing)
  (CallFunction|OrangeDancing))

(fn ConstructionScript)

(fn GreenDancing
  (bind _greenplayer (Variables|Default|GetGreenPlayer))
  (bind _skeletalmeshcomponent (Variables|/Script/Engine.SkeletalMeshActor|GetSkeletalMeshComponent _greenplayer))
  (if (.IsHuman (Utilities|Struct|BreakPlayerStruct (Utilities|Array|Get(acopy) (Variables|/Game/MyGameInstance.MyGameInstance_C|GetPlayers (Variables|Default|GetGameInstance)) 1)))
    (if (not (Variables|Default|GetGreenIsDancing))
      (Variables|Default|SetGreenIsDancing true)
      (Components|Animation|PlayAnimation _skeletalmeshcomponent "/Game/MainMenu/Robot_Hip_Hop_Dance__1_.Robot_Hip_Hop_Dance__1_" true))
    (elif (Variables|Default|GetGreenIsDancing)
      (Variables|Default|SetGreenIsDancing false)
      (Components|Animation|PlayAnimation _skeletalmeshcomponent "/Game/Characters/AnimationsSequences/Breathing_Idle.Breathing_Idle" true))))

(fn RedDancing
  (bind _redplayer (Variables|Default|GetRedPlayer))
  (bind _skeletalmeshcomponent (Variables|/Script/Engine.SkeletalMeshActor|GetSkeletalMeshComponent _redplayer))
  (if (.IsHuman (Utilities|Struct|BreakPlayerStruct (Utilities|Array|Get(acopy) (Variables|/Game/MyGameInstance.MyGameInstance_C|GetPlayers (Variables|Default|GetGameInstance)) 2)))
    (if (not (Variables|Default|GetRedIsDancing))
      (Variables|Default|SetRedIsDancing true)
      (Components|Animation|PlayAnimation _skeletalmeshcomponent "/Game/MainMenu/Rumba_Dancing__1_.Rumba_Dancing__1_" true))
    (elif (Variables|Default|GetRedIsDancing)
      (Variables|Default|SetRedIsDancing false)
      (Components|Animation|PlayAnimation _skeletalmeshcomponent "/Game/Characters/AnimationsSequences/Breathing_Idle.Breathing_Idle" true))))

(fn OrangeDancing
  (bind _orangeplayer (Variables|Default|GetOrangePlayer))
  (bind _skeletalmeshcomponent (Variables|/Script/Engine.SkeletalMeshActor|GetSkeletalMeshComponent _orangeplayer))
  (if (.IsHuman (Utilities|Struct|BreakPlayerStruct (Utilities|Array|Get(acopy) (Variables|/Game/MyGameInstance.MyGameInstance_C|GetPlayers (Variables|Default|GetGameInstance)) 3)))
    (if (not (Variables|Default|GetOrangeIsDancing))
      (Variables|Default|SetOrangeIsDancing true)
      (Components|Animation|PlayAnimation _skeletalmeshcomponent "/Game/MainMenu/Swing_Dancing.Swing_Dancing" true))
    (elif (Variables|Default|GetOrangeIsDancing)
      (Variables|Default|SetOrangeIsDancing false)
      (Components|Animation|PlayAnimation _skeletalmeshcomponent "/Game/Characters/AnimationsSequences/Breathing_Idle.Breathing_Idle" true))))