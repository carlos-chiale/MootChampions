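; BP_BouncePile is a bounce obstacle in the PushAway game that stands on a BP_Platform and knocks players on contact.
; On actor overlap it launches a BP_PushAwayPlayer by that player's velocity times BounceVelocity, added to current velocity, and plays the Rebote sound.
; Tick polls the capsule's overlaps and destroys the pile once it touches no platform.
; BeginPlay caches the game manager, which is otherwise unused here.
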(event EventBeginPlay
  (bind _returnvalue (Actor|GetActorOfClass "/Game/PushAway/Blueprints/BP_GameManagerPushAway.BP_GameManagerPushAway_C"))
  (Variables|Default|SetGameManager _returnvalue))

(event Collision|EventActorBeginOverlap
  (params (OtherActor :type Actor%20Object%20Reference))
  (bind _asbp_push_away_player (Utilities|Casting|CastToBP_PushAwayPlayer OtherActor))
  (Character|LaunchCharacter _asbp_push_away_player (* (Transformation|GetVelocity _asbp_push_away_player) (Variables|Default|GetBounceVelocity)) false false)
  (Audio|PlaySoundatLocation "/Game/Sound/Rebote.Rebote" (Transformation|GetActorLocation self) "0, 0, 0" 1.0 1.0 0.0 0 0 0))

(event EventTick
  (params (DeltaSeconds :type Float%20%28single-precision%29))
  (if (== (Utilities|Array|Length (Collision|GetOverlappingActors (Variables|Default|GetCapsule) "/Game/PushAway/Blueprints/BP_Platform.BP_Platform_C" :!class /Script/Engine.PrimitiveComponent)) 0)
    (Actor|DestroyActor)))

(fn ConstructionScript)