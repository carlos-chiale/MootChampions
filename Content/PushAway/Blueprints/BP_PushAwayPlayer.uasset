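; Player character for the PushAway game, which moves, tackles to launch other players, and reports its death to the game manager when destroyed.
; Jump sets a tackle flag, and overlaps on TackleCollision then launch the other player at four times this character's velocity.
; Looping one-second timers count down speed-boost and stun timers, with stun blocking movement.
; It also selects a colored mesh by player index and opens the pause menu.
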(event OnComponentBeginOverlap(TackleCollision)
  (params (OverlappedComponent :type Primitive%20Component%20Object%20Reference) (OtherActor :type Actor%20Object%20Reference) (OtherComp :type Primitive%20Component%20Object%20Reference) (OtherBodyIndex :type Integer) (bFromSweep :type Boolean) (SweepResult :type Hit%20Result%20Structure%20%28by%20ref%29))
  ;[1 1 1] Tackle
  (bind _asbp_push_away_player (Utilities|Casting|CastToBP_PushAwayPlayer OtherActor))
  (if (Variables|Default|GetIsTackling)
    (Character|LaunchCharacter _asbp_push_away_player (* (Variables|/Script/Engine.MovementComponent|GetVelocity (Variables|Character|GetCharacterMovement)) 4) false false)))

(event EventTick
  (params (DeltaSeconds :type Float%20%28single-precision%29)))

(event Collision|EventActorBeginOverlap
  (params (OtherActor :type Actor%20Object%20Reference)))

(event EventBeginPlay
  (bind _returnvalue (Actor|GetActorOfClass "/Game/PushAway/Blueprints/BP_GameManagerPushAway.BP_GameManagerPushAway_C"))
  (Variables|Default|SetGameManager _returnvalue)
  (Utilities|Time|SetTimerbyFunctionName 0 "DecrementWhileSpeedIncreased" 1.0 true)
  (Utilities|Time|SetTimerbyFunctionName 0 "DecrementWhileStunning" 1.0 true))

(event EventDestroyed
  (Default|MarkasDead (Variables|Default|GetGameManager) (Variables|Default|GetIndex)))

(event Input|ActionEvents|InputActionJump
  (params (Key :type Key%20Structure))
  ;[1 1 1] Tackle
  (:Pressed
    (if (not (Variables|Default|GetIsTackling))
      (Variables|Default|SetIsTackling true))))

(event Input|AxisEvents|InputAxisMoveForward
  (params (AxisValue :type Float%20%28single-precision%29))
  ;[1 1 1] Movement
  (if (not (Variables|Default|GetIsStunt))
    (Pawn|Input|AddMovementInput "90.000000, 0, 0" AxisValue false)))

(event Input|AxisEvents|InputAxisMoveRight
  (params (AxisValue :type Float%20%28single-precision%29))
  ;[1 1 1] Movement
  (if (not (Variables|Default|GetIsStunt))
    (Pawn|Input|AddMovementInput "0.000000,90.000000, 0" AxisValue false)))

(event Input|KeyboardEvents|P
  (params (Key :type Key%20Structure))
  (bind _returnvalue (Game|GetPlayerController 0))
  (:Pressed
    (Variables|/Script/Engine.PlayerController|SetbShowMouseCursor _returnvalue true)
    (bind _returnvalue_2 (UserInterface|CreateWidget "/Game/PauseMenu/W_PauseMenu.W_PauseMenu_C"))
    (UserInterface|Viewport|AddtoViewport _returnvalue_2 0)
    (Game|SetGamePaused true)
    (Input|SetInputModeUIOnly _returnvalue _returnvalue_2 "DoNotLock")))

(event Input|KeyboardEvents|Escape
  (params (Key :type Key%20Structure))
  (bind _returnvalue (Game|GetPlayerController 0))
  (:Pressed
    (Variables|/Script/Engine.PlayerController|SetbShowMouseCursor _returnvalue true)
    (bind _returnvalue_2 (UserInterface|CreateWidget "/Game/PauseMenu/W_PauseMenu.W_PauseMenu_C"))
    (UserInterface|Viewport|AddtoViewport _returnvalue_2 0)
    (Game|SetGamePaused true)
    (Input|SetInputModeUIOnly _returnvalue _returnvalue_2 "DoNotLock")))

(fn ConstructionScript)

(fn SetPlayerandColorbyIndex
  (Class|SkinnedMeshComponent|SetSkeletalMesh (Variables|Character|GetMesh) (Utilities|Select :Index (Variables|Default|GetIndex) :Option%200 "/Game/Characters/CharacterTPose/BlueCharacter/TPoseBlueCharacter.TPoseBlueCharacter" :Option%201 "/Game/Characters/CharacterTPose/GreenCharacter/TPoseGreenCharacter.TPoseGreenCharacter" :Option%202 "/Game/Characters/CharacterTPose/RedCharacter/TPoseRedCharacter.TPoseRedCharacter" :Option%203 "/Game/Characters/CharacterTPose/YellowCharacter/TPoseYellowCharacter.TPoseYellowCharacter") true))

(fn IncrementVelocity
  (Variables|/Script/Engine.CharacterMovementComponent|SetMaxWalkSpeed (Variables|Character|GetCharacterMovement) 1.2e+03)
  (Variables|Default|SetIsSpeedIncremented true)
  (Variables|Default|SetTimeToPutMaxSpeedNormal 5))

(fn DecrementWhileSpeedIncreased
  (if (Variables|Default|GetIsSpeedIncremented)
    (Variables|Default|SetTimeToPutMaxSpeedNormal (- (Variables|Default|GetTimeToPutMaxSpeedNormal) 1))))

(fn DecrementWhileStunning
  (if (Variables|Default|GetIsStunt)
    (Variables|Default|SetTimeToUnstunt (- (Variables|Default|GetTimeToUnstunt) 1))))