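; Game manager for the PushAway minigame, running the shrinking arena, eliminations and end of match.
; At BeginPlay it scatters piles over the platform, retrying random points until a sphere overlap finds no nearby BP_BouncePile.
; A one-second timer drives periodic shrinking of the platform's X/Y scale.
; MarkAsDead fills the ranking from last place; after three deaths, Tick copies it to MyGameInstance, pauses and shows the win widget.
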(event EventBeginPlay
  (Variables|Tosetup|SetAuxTimeToReducePlatform (Variables|Tosetup|GetTimeToReducePlatform))
  (Utilities|Time|SetTimerbyFunctionName 0 "Decrement" 1.0 true)
  (CallFunction|SetPiles))

(event EventTick
  (params (DeltaSeconds :type Float%20%28single-precision%29))
  (bind _returnvalue (Game|GetPlayerController 0))
  (CallFunction|ReducePlatform)
  (if (Variables|Default|GetGameFinished)
    (Variables|Default|SetFinalRanking (Variables|Default|GetRankingOrder))
    (bind _asmy_game_instance (Utilities|Casting|CastToMyGameInstance (Game|GetGameInstance)))
    (for (_array_element _array_index) (Variables|Default|GetFinalRanking)
      (Utilities|Array|SetArrayElem (Variables|/Game/MyGameInstance.MyGameInstance_C|GetLastGameRank _asmy_game_instance) _array_index _array_element))
    (Input|SetInputModeGameandUI _returnvalue 0 "DoNotLock" false)
    (Variables|/Script/Engine.PlayerController|SetbShowMouseCursor _returnvalue true)
    (Game|SetGamePaused true)
    (bind _returnvalue_2 (UserInterface|CreateWidget "/Game/PaintTheFloor/Blueprints/UI/W_Win.W_Win_C"))
    (UserInterface|Viewport|AddtoViewport _returnvalue_2 0)))

(fn ConstructionScript)

(fn Decrement
  (Variables|Tosetup|SetTimeInSeconds (- (Variables|Tosetup|GetTimeInSeconds) 1))
  (Variables|Tosetup|SetAuxTimeToReducePlatform (- (Variables|Tosetup|GetAuxTimeToReducePlatform) 1)))

(fn MarkasDead
  (params (PlayerIndex :type Integer))
  (Utilities|Array|SetArrayElem (Variables|Default|GetIsDead) PlayerIndex true)
  (Variables|Default|SetNumberOfDeaths (+ (Variables|Default|GetNumberOfDeaths) 1))
  (Utilities|Array|SetArrayElem (Variables|Default|GetRankingOrder) (Variables|Default|GetAuxRankingIndex) PlayerIndex)
  (Variables|Default|SetAuxRankingIndex (- (Variables|Default|GetAuxRankingIndex) 1))
  (if (== (Variables|Default|GetNumberOfDeaths) 3)
    (for (_array_element _array_index) (Variables|Default|GetIsDead)
      (if (not _array_element)
        (Utilities|Array|SetArrayElem (Variables|Default|GetRankingOrder) (Variables|Default|GetAuxRankingIndex) _array_index)))
    (Variables|Default|SetGameFinished true)))

(fn ReducePlatform
  (bind _platform (Variables|Default|GetPlatform))
  (bind _platformreduction (Variables|Tosetup|GetPlatformReduction))
  (bind _returnvalue (Transformation|GetActorScale3D _platform))
  (if (== (Variables|Tosetup|GetAuxTimeToReducePlatform) 0)
    (Variables|Tosetup|SetAuxTimeToReducePlatform (Variables|Tosetup|GetTimeToReducePlatform))
    (Transformation|SetActorScale3D _platform (Math|Vector|MakeVector (- (.x _returnvalue) _platformreduction) (- (.y _returnvalue) _platformreduction) (.z _returnvalue)))))

(fn SetPiles
  (bind _platform (Variables|Default|GetPlatform))
  (bind _origin (Variables|/Game/PushAway/Blueprints/BP_Platform.BP_Platform_C|GetOrigin _platform))
  (bind _box (Variables|/Game/PushAway/Blueprints/BP_Platform.BP_Platform_C|GetBox _platform))
  (bind _returnvalue (Transformation|GetWorldLocation _origin))
  (bind _returnvalue_2 (Components|Box|GetScaledBoxExtent _box))
  (bind _returnvalue_3 (Math|Random|RandomPointinBoundingBox _returnvalue _returnvalue_2))
  (bind (_x _y) (Math|Vector|BreakVector _returnvalue_3))
  (while (> (Variables|Tosetup|GetAmountOfPiles) 0)
    (LocalVariables|SetIsOkToAdd false)
    (while (not (LocalVariables|GetIsOkToAdd))
      (bind _output_get (LocalVariables|SetLocationAux (Math|Vector|MakeVector _x _y 134.0)))
      (bind _outactors (Collision|SphereOverlapActors _output_get (Variables|Tosetup|GetDistanceBetweenPiles) (Utilities|Array|MakeArray "ObjectTypeQuery2") "/Game/PushAway/Blueprints/BP_BouncePile.BP_BouncePile_C"))
      (if (not (> (Utilities|Array|Length _outactors) 0))
        (LocalVariables|SetIsOkToAdd true)))
    (Game|SpawnActorfromClass "/Game/PushAway/Blueprints/BP_BouncePile.BP_BouncePile_C" (Math|Transform|MakeTransform (LocalVariables|GetLocationAux)) "Undefined" 0 0)
    (Variables|Tosetup|SetAmountOfPiles (- (Variables|Tosetup|GetAmountOfPiles) 1))))